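; Human_BP is a player-controlled human pawn that handles basic movement and look input.
; Forward, backward, left and right axis events add movement input along forward or right vectors derived from control yaw only.
; LeftTurn and UpTurn feed controller yaw and pitch.
; UpTurn also plays a non-looping walk animation directly on the mesh every time its axis event fires, regardless of axis value.
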(event `InputAxis|BackwardMovement`
  (params (AxisValue :type "Float (single-precision)"))
  (`self.AddMovementInput` (`KismetMathLibrary.GetForwardVector` (`KismetMathLibrary.MakeRotator` 0.0 0.0 (.yaw (`self.GetControlRotation`)))) AxisValue))

(event `self.ReceiveTick`
  (params (DeltaSeconds :type "Float (single-precision)")))

(event `InputAxis|ForwardMovement`
  (params (AxisValue :type "Float (single-precision)"))
  (`self.AddMovementInput` (`KismetMathLibrary.GetForwardVector` (`KismetMathLibrary.MakeRotator` 0.0 0.0 (.yaw (`self.GetControlRotation`)))) AxisValue))

(event `InputAxis|LeftMovement`
  (params (AxisValue :type "Float (single-precision)"))
  (`self.AddMovementInput` (`KismetMathLibrary.GetRightVector` (`KismetMathLibrary.MakeRotator` 0.0 0.0 (.yaw (`self.GetControlRotation`)))) AxisValue))

(event `InputAxis|RightMovement`
  (params (AxisValue :type "Float (single-precision)"))
  (`self.AddMovementInput` (`KismetMathLibrary.GetRightVector` (`KismetMathLibrary.MakeRotator` 0.0 0.0 (.yaw (`self.GetControlRotation`)))) AxisValue))

(event `InputAxis|LeftTurn`
  (params (AxisValue :type "Float (single-precision)"))
  (`self.AddControllerYawInput` AxisValue))

(event `InputAxis|UpTurn`
  (params (AxisValue :type "Float (single-precision)"))
  (`self.AddControllerPitchInput` AxisValue)
  (`SkeletalMeshComponent.PlayAnimation` (`self.Mesh`) "/Engine/Tutorial/SubEditors/TutorialAssets/Character/Tutorial_Walk_Fwd.Tutorial_Walk_Fwd" false))

(event `self.Mesh.OnAnimInitialized`)

(fn `UserConstructionScript`)